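; BP_Drawer is an interactable drawer the player can get into and out of, moving a Door component as they do.
; Interact toggles an Inside flag and teleports player 0 to the REFInside or REFOutside transform.
; The Door snaps to zero rotation on entry and swings open on exit, with no animation.
; The Trigget overlap only prints a debug greeting for BP_FirstPersonCharacter and does not gate interaction.
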(event `self.Trigget.OnComponentBeginOverlap`
  (params (OverlappedComponent :type "PrimitiveComponent Object Reference") (OtherActor :type "Actor Object Reference") (OtherComp :type "PrimitiveComponent Object Reference") (OtherBodyIndex :type Integer) (bFromSweep :type Boolean) (SweepResult :type "HitResult Structure (by ref)"))
  (cast `/Game/ThirdPerson/Blueprints/BP_FirstPersonCharacter` OtherActor)
  (`KismetSystemLibrary.PrintString` "Hello"))

(event `/Game/Blueprints/BPI_Interaction.Interact`
  (bind (_returnvalue_location _returnvalue_rotation) (`KismetMathLibrary.BreakTransform` (`SceneComponent.K2_GetComponentToWorld` (`self.REF Inside`))))
  (bind (_returnvalue_location_2 _returnvalue_rotation_2) (`KismetMathLibrary.BreakTransform` (`SceneComponent.K2_GetComponentToWorld` (`self.REF Outside`))))
  (if (not (`self.Inside`))
    (set `self.Inside` true)
    (`self.K2_SetActorTransform` (`GameplayStatics.GetPlayerCharacter` 0) (`KismetMathLibrary.MakeTransform` _returnvalue_location _returnvalue_rotation) false false)
    (`SceneComponent.K2_SetRelativeRotation` :`self` (`self.Door`))
    (else
      (set `self.Inside` false)
      (`self.K2_SetActorTransform` (`GameplayStatics.GetPlayerCharacter` 0) (`KismetMathLibrary.MakeTransform` _returnvalue_location_2 _returnvalue_rotation_2) false false)
      (`SceneComponent.K2_SetRelativeRotation` (`self.Door`) (struct :`Yaw` 110.0) false false))))

(fn `UserConstructionScript`)